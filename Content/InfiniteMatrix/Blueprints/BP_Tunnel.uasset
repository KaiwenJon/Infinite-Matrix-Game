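; BP_Tunnel is a tunnel segment with a spinning holed wall and optional tumbling health pack and enemy pickups.
; Passing the trigger raises BP_Player's score and speed, while hitting the wall cuts health and speed, triggering restart at zero health.
; Either event has TunnelSpawner spawn another tunnel and destroys this one.
; Randomize functions vary wall mesh and roll, and offset or remove pickups; enemy contact damages without a death check.
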(event `self.ReceiveBeginPlay`)

(event `self.ReceiveTick`
  (params (DeltaSeconds :type "Float (single-precision)"))
  (bind _returnvalue (* DeltaSeconds 50.0))
  (bind _healthpack (`self.HealthPack`))
  (bind _enemy (`self.Enemy`))
  (`SceneComponent.K2_AddLocalRotation` (`self.WallMesh`) (`KismetMathLibrary.MakeRotator` (* DeltaSeconds (`self.RotateSpeed`))) false false)
  (`|ExecutionSequence`
    (:`then_0`
      (`/Engine/EditorBlueprintResources/StandardMacros.IsValid` _enemy
        (:`Is Valid`
          (`SceneComponent.K2_AddLocalRotation` _enemy (`KismetMathLibrary.MakeRotator` _returnvalue _returnvalue _returnvalue) false false))))
    (:`then_1`
      (`/Engine/EditorBlueprintResources/StandardMacros.IsValid` _healthpack
        (:`Is Valid`
          (`SceneComponent.K2_AddLocalRotation` _healthpack (`KismetMathLibrary.MakeRotator` _returnvalue _returnvalue _returnvalue) false false))))))

(event `self.TriggerZone.OnComponentBeginOverlap`
  (params (OverlappedComponent :type "PrimitiveComponent Object Reference") (OtherActor :type "Actor Object Reference") (OtherComp :type "PrimitiveComponent Object Reference") (OtherBodyIndex :type Integer) (bFromSweep :type Boolean) (SweepResult :type "HitResult Structure (by ref)"))
  (bind _asbp_player (cast `/Game/InfiniteMatrix/Blueprints/BP_Player` OtherActor))
  (`/Game/InfiniteMatrix/Blueprints/BP_TunnelSpawner.SpawnTunnelAtSpawnPoint` (`self.TunnelSpawner`))
  (`self.K2_DestroyActor`)
  (set `/Game/InfiniteMatrix/Blueprints/BP_Player.Score` (+ (`/Game/InfiniteMatrix/Blueprints/BP_Player.Score` _asbp_player) 1) _asbp_player)
  (set `/Game/InfiniteMatrix/Blueprints/BP_Player.ForwardSpeed` (`KismetMathLibrary.FClamp` (+ (`/Game/InfiniteMatrix/Blueprints/BP_Player.ForwardSpeed` _asbp_player) 100.0) 2000.0 3000.0) _asbp_player))

(event `self.WallMesh.OnComponentHit`
  (params (HitComponent :type "PrimitiveComponent Object Reference") (OtherActor :type "Actor Object Reference") (OtherComp :type "PrimitiveComponent Object Reference") (NormalImpulse :type "Vector Structure") (Hit :type "HitResult Structure (by ref)"))
  (bind _asbp_player (cast `/Game/InfiniteMatrix/Blueprints/BP_Player` OtherActor))
  (set `/Game/InfiniteMatrix/Blueprints/BP_Player.Health` (`KismetMathLibrary.FClamp` (- (`/Game/InfiniteMatrix/Blueprints/BP_Player.Health` _asbp_player) 20.0) 0.0 100.0) _asbp_player)
  (set `/Game/InfiniteMatrix/Blueprints/BP_Player.ForwardSpeed` (`KismetMathLibrary.FClamp` (- (`/Game/InfiniteMatrix/Blueprints/BP_Player.ForwardSpeed` _asbp_player) 300.0) 2000.0 3000.0) _asbp_player)
  (`/Game/InfiniteMatrix/Blueprints/BP_TunnelSpawner.SpawnTunnelAtSpawnPoint` (`self.TunnelSpawner`))
  (`self.K2_DestroyActor`)
  (if (== (`/Game/InfiniteMatrix/Blueprints/BP_Player.Health` _asbp_player) 0.0)
    (set `/Game/InfiniteMatrix/Blueprints/BP_Player.IsDead` true _asbp_player)
    (`/Game/InfiniteMatrix/Blueprints/BP_Player.DisplayRestart` _asbp_player)))

(event `self.HealthPack.OnComponentBeginOverlap`
  (params (OverlappedComponent :type "PrimitiveComponent Object Reference") (OtherActor :type "Actor Object Reference") (OtherComp :type "PrimitiveComponent Object Reference") (OtherBodyIndex :type Integer) (bFromSweep :type Boolean) (SweepResult :type "HitResult Structure (by ref)"))
  (bind _asbp_player (cast `/Game/InfiniteMatrix/Blueprints/BP_Player` OtherActor))
  (`KismetSystemLibrary.PrintString` "Bump!")
  (`ActorComponent.K2_DestroyComponent` (`self.HealthPack`))
  (set `/Game/InfiniteMatrix/Blueprints/BP_Player.Health` (`KismetMathLibrary.FClamp` (+ (`/Game/InfiniteMatrix/Blueprints/BP_Player.Health` _asbp_player) 10.0) 0.0 100.0) _asbp_player))

(event `self.Enemy.OnComponentBeginOverlap`
  (params (OverlappedComponent :type "PrimitiveComponent Object Reference") (OtherActor :type "Actor Object Reference") (OtherComp :type "PrimitiveComponent Object Reference") (OtherBodyIndex :type Integer) (bFromSweep :type Boolean) (SweepResult :type "HitResult Structure (by ref)"))
  (bind _asbp_player (cast `/Game/InfiniteMatrix/Blueprints/BP_Player` OtherActor))
  (`ActorComponent.K2_DestroyComponent` (`self.Enemy`))
  (`KismetSystemLibrary.PrintString` "Stone")
  (set `/Game/InfiniteMatrix/Blueprints/BP_Player.Health` (`KismetMathLibrary.FClamp` (- (`/Game/InfiniteMatrix/Blueprints/BP_Player.Health` _asbp_player) 20.0) 0.0 100.0) _asbp_player))

(fn `RandomizeEnemy`
  (bind _returnvalue (`KismetMathLibrary.RandomFloatInRange` -300.0 300.0))
  (if (>= (`KismetMathLibrary.RandomFloatInRange` 0.0 1.0) 0.5)
    (`SceneComponent.K2_AddLocalOffset` (`self.Enemy`) (`KismetMathLibrary.MakeVector` 0.0 _returnvalue _returnvalue) false false)
    (else
      (`ActorComponent.K2_DestroyComponent` (`self.Enemy`)))))

(fn `RandomizePack`
  (bind _returnvalue (`KismetMathLibrary.RandomFloatInRange` -300.0 300.0))
  (if (> (`KismetMathLibrary.RandomFloatInRange` 0.0 1.0) 0.5)
    (`SceneComponent.K2_AddLocalOffset` (`self.HealthPack`) (`KismetMathLibrary.MakeVector` 0.0 _returnvalue _returnvalue) false false)
    (else
      (`ActorComponent.K2_DestroyComponent` (`self.HealthPack`)))))

(fn `RandomizeWall`
  (`StaticMeshComponent.SetStaticMesh` (`self.WallMesh`) (select `int` (`KismetMathLibrary.RandomIntegerInRange` 0 3) :`0` "/Game/InfiniteMatrix/Meshes/SM_Hole_01.SM_Hole_01" :`1` "/Game/InfiniteMatrix/Meshes/SM_Hole_02.SM_Hole_02" :`2` "/Game/InfiniteMatrix/Meshes/SM_Hole_03.SM_Hole_03" :`3` "/Game/InfiniteMatrix/Meshes/SM_Hole_04.SM_Hole_04" :!type "StaticMesh Object Reference"))
  (`SceneComponent.K2_AddLocalRotation` (`self.WallMesh`) (`KismetMathLibrary.MakeRotator` (`KismetMathLibrary.RandomFloatInRange` 0.0 360.0)) false false))

(fn `UserConstructionScript`)